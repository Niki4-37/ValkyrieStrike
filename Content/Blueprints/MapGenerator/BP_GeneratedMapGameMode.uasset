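; Game mode for generated maps that builds the level at play start and puts the player in a vehicle.
; On BeginPlay it spawns BP_MapGenerator at the origin with a set tile size, then waits on a fixed delay rather than a completion signal.
; It then spawns BP_DefaultWeeledVehicle at the first PlayerStart found and has player controller 0 possess it; if none exists, no vehicle is spawned.
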(event EventBeginPlay
  (Game|SpawnActorfromClass "/Game/Blueprints/MapGenerator/BP_MapGenerator.BP_MapGenerator_C" (Math|Transform|MakeTransform "0, 0, 0") "Undefined" 0 5 5 0 1e+03 0 0)
  (Utilities|FlowControl|Delay 1.0)
  (bind _outactors (Actor|GetAllActorsOfClass "/Script/Engine.PlayerStart"))
  (if (Math|Conversions|ToBoolean(Integer) (Utilities|Array|Length _outactors))
    (bind _returnvalue (Game|SpawnActorfromClass "/Game/Blueprints/Player/BP_DefaultWeeledVehicle.BP_DefaultWeeledVehicle_C" (Math|Transform|MakeTransform (Transformation|GetActorLocation (Utilities|Array|Get(acopy) _outactors))) "Undefined" 0 0))
    (Pawn|Possess (Game|GetPlayerController 0) _returnvalue)))

(event EventTick
  (params (DeltaSeconds :type Float%20%28single-precision%29)))

(fn ConstructionScript)