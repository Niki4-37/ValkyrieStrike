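; BP_MapGenerator builds a tiled map at BeginPlay by instancing streaming levels across a NumX by NumY grid.
; Each cell checks SpecialTiles for matching coordinates, using that entry's level names if found and the default LevelNames otherwise.
; A random level from the chosen list becomes a uniquely named streaming instance, offset by TileSize and set loaded and visible.
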(event EventBeginPlay
  (for _index (range 0 (- (Variables|Default|GetNumX) 1))
    (Variables|Default|SetXCount _index)
    (for _index_2 (range 0 (- (Variables|Default|GetNumY) 1))
      (Variables|Default|SetYCount _index_2)
      (bind (_bisfound _tilename) (CallFunction|CheckSpecialTile))
      (if _bisfound
        (CallFunction|CreateandPlaceLevel _tilename)
        (else
          (CallFunction|CreateandPlaceLevel (Variables|Default|GetLevelNames)))))))

(fn ConstructionScript)

(fn CreateandPlaceLevel
  (params (InputPin :type Array%20of%20Names))
  (bind _returnvalue (Class|LevelStreaming|CreateInstance (Class|GameplayStatics|GetStreamingLevel (Utilities|Array|Get(acopy) InputPin (Math|Random|RandomIntegerinRange 0 (Utilities|Array|LastIndex InputPin)))) (Utilities|String|Append (Utilities|String|ToString(Integer) (Variables|Default|GetXCount)) "x" (Utilities|String|ToString(Integer) (Variables|Default|GetYCount)))))
  (Variables|/Script/Engine.LevelStreaming|SetLevelTransform _returnvalue (Math|Transform|MakeTransform (Math|Vector|MakeVector (* (Variables|Default|GetXCount) (Variables|Default|GetTileSize)) (* (Variables|Default|GetYCount) (Variables|Default|GetTileSize)) 0.0)))
  (Variables|/Script/Engine.LevelStreaming|SetbShouldBeLoaded _returnvalue true)
  (Variables|/Script/Engine.LevelStreaming|SetbShouldBeVisible _returnvalue true))

(fn CheckSpecialTile
  (LocalVariables|SetbSpecialTileFound false)
  (for _array_element (Variables|Default|GetSpecialTiles)
    (if (not (LocalVariables|GetbSpecialTileFound))
      (LocalVariables|SetbSpecialTileFound (and (== (.X (Math|Vector|BreakVector (.Coordinates (Utilities|Struct|BreakFSpecialTile _array_element)))) (Math|Conversions|ToFloat(Integer) (Variables|Default|GetXCount))) (== (.Y (Math|Vector|BreakVector (.Coordinates (Utilities|Struct|BreakFSpecialTile _array_element)))) (Math|Conversions|ToFloat(Integer) (Variables|Default|GetYCount)))))
      (LocalVariables|SetSpecialTileName (.LevelName (Utilities|Struct|BreakFSpecialTile _array_element)))))
  (return (LocalVariables|GetbSpecialTileFound) (LocalVariables|GetSpecialTileName)))