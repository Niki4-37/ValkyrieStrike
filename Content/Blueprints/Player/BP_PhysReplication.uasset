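; Actor component that replicates a simulated physics body from server to clients, auto-targeting the owner's root when default.
; The server publishes transform and velocities each tick, optionally toggling ticking and net update frequency on physics wake/sleep.
; On replication, clients teleport the body, easing small location errors by distance-scaled lerp.
; They also set angular velocity, but linear velocity is fed the replicated Location field.
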(event Custom|SimulationWake
  (params (WakingComponent :type Primitive%20Component%20Object%20Reference) (BoneName :type Name))
  (bind _owner (Variables|Default|GetOwner))
  (bind _wakeupdatefrequency (Variables|Default|GetWakeUpdateFrequency))
  (if (Variables|Default|GetIsServer)
    (Variables|/Script/Engine.Actor|SetNetUpdateFrequency _owner _wakeupdatefrequency)
    (Variables|/Script/Engine.Actor|SetMinNetUpdateFrequency _owner (* _wakeupdatefrequency (Variables|Default|GetMinUpdateMultiplier)))
    (Networking|ForceNetUpdate _owner)
    (Components|Tick|SetComponentTickEnabled true)))

(event Custom|SimulationSleep
  (params (SleepingComponent :type Primitive%20Component%20Object%20Reference) (BoneName :type Name))
  (bind _sleepupdatefrequency (Variables|Default|GetSleepUpdateFrequency))
  (bind _owner (Variables|Default|GetOwner))
  (if (Variables|Default|GetIsServer)
    (Variables|/Script/Engine.Actor|SetNetUpdateFrequency _owner _sleepupdatefrequency)
    (Variables|/Script/Engine.Actor|SetMinNetUpdateFrequency _owner (* _sleepupdatefrequency (Variables|Default|GetMinUpdateMultiplier)))
    (Components|Tick|SetComponentTickEnabled false)))

(event EventBeginPlay
  (bind _returnvalue (Components|GetOwner))
  ;[1 1 1] Add Data
  (Utilities|IsValid _returnvalue
    (:Is%20Valid
      (Variables|Default|SetOwner _returnvalue)
      (Variables|Default|SetIsServer (Ability|HasAuthority _returnvalue))
      ;[1 1 1] Used by default
      (if (Variables|Default|GetIsDefault)
        (bind _asprimitive_component (Utilities|Casting|CastToPrimitiveComponent (Variables|/Script/Engine.Actor|GetRootComponent (Variables|Default|GetOwner))))
        (if (Physics|IsSimulatingPhysics _asprimitive_component "None")
          (CallFunction|SetSyncComponent _asprimitive_component true))))))

(event EventTick
  (params (DeltaSeconds :type Float%20%28single-precision%29))
  (bind _physcomponent (Variables|Default|GetPhysComponent))
  (bind _returnvalue (Transformation|GetWorldTransform _physcomponent))
  (if (Variables|Default|GetIsServer)
    (Variables|Default|SetRepData (Utilities|Struct|MakeS_MoveReplicationData (.location _returnvalue) (.rotation _returnvalue) (Transformation|GetComponentVelocity _physcomponent) (Physics|GetPhysicsAngularVelocityinDegrees _physcomponent "None")))))

(fn SetSyncComponent
  (params (SimulatedComponent :type Primitive%20Component%20Object%20Reference) (IsActive :type Boolean))
  (Variables|Default|SetPhysComponent SimulatedComponent)
  (Utilities|FlowControl|Sequence
    (:then_0
      (if IsActive
        (if (Variables|Default|GetIsServer)
          (Components|Tick|SetComponentTickEnabled true))))
    (:then_1
      (if (Variables|Default|GetAllowSyncFrequencyChanging)
        (EventDispatchers|BindEventtoOnComponentWake (Variables|Default|GetPhysComponent) (EventDispatchers|CreateEvent :!event Custom|SimulationWake))
        (EventDispatchers|BindEventtoOnComponentSleep (Variables|Default|GetPhysComponent) (EventDispatchers|CreateEvent :!event Custom|SimulationSleep))))))

(fn OnRepRepData
  (bind _physcomponent (Variables|Default|GetPhysComponent))
  (bind _repdata (Variables|Default|GetRepData))
  (bind _physcomponent_2 (Variables|Default|GetPhysComponent))
  (bind _returnvalue (Transformation|GetWorldLocation _physcomponent_2))
  (if (not (Variables|Default|GetIsServer))
    (Utilities|IsValid (Variables|Default|GetPhysComponent)
      (:Is%20Valid
        ;[1 1 1] Velocity
        (Physics|SetPhysicsLinearVelocity _physcomponent (.location _repdata) false "None")
        (Class|PrimitiveComponent|SetPhysicsAngularVelocityinDegrees _physcomponent (.angularvelocity _repdata) false "None")
        (Utilities|FlowControl|Sequence
          (:then_0
            ;[1 1 1] Compute Location
            (if (== (Variables|Default|GetLocationInaccuracy) 0.0)
              (Variables|Default|SetRep%20Data%20Location (.location (Variables|Default|GetRepData)))
              (else
                (Variables|Default|SetRep%20Data%20Location (Math|Vector|Lerp(Vector) _returnvalue (.location (Variables|Default|GetRepData)) (/ (Math|Float|Clamp(Float) (Math|Vector|VectorLength (- _returnvalue (.location (Variables|Default|GetRepData)))) 0.0 (Variables|Default|GetLocationInaccuracy)) (Variables|Default|GetLocationInaccuracy)))))))
          (:then_1
            (Transformation|SetWorldLocationAndRotation (Variables|Default|GetPhysComponent) (Variables|Default|GetRep%20Data%20Location) (.rotation (Variables|Default|GetRepData)) false true)))))))